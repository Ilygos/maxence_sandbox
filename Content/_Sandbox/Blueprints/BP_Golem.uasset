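; BP_Golem is a sandbox golem Blueprint with a skeletal mesh that can be activated and visually marked as locked.
; Activate casts the mesh's animation instance to ABP_Golem and calls its Roar.
; ToggleLock switches custom depth rendering on the mesh with a stencil value, presumably for a lock-on highlight in post-processing.
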(event Custom|Activate
  (bind _asabp_golem (Utilities|Casting|CastToABP_Golem (Components|SkeletalMesh|GetAnimInstance (Variables|Character|GetMesh))))
  (Default|Roar _asabp_golem))

(event EventToggleLock
  (params (IsLocked :type Boolean))
  (bind _mesh (Variables|Character|GetMesh))
  (if IsLocked
    (Rendering|SetRenderCustomDepth _mesh true)
    (Rendering|SetCustomDepthStencilValue _mesh 2)
    (else
      (Rendering|SetRenderCustomDepth _mesh false)
      (Rendering|SetCustomDepthStencilValue _mesh 0))))

(fn ConstructionScript)