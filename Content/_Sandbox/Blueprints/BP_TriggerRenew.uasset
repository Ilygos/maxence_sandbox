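; BP_TriggerRenew is a trigger actor that fades the global IsAbsorbing effect parameter in and out as the player character enters and leaves it.
; Overlap events read the current value from the C_EffectsParameters collection and set the fade direction, with exit also playing DoorSequence.
; Tick steps the value by IncrementValue in that direction, clamps it between zero and one, and writes it back every frame.
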(event EventTick
  (params (DeltaSeconds :type Float%20%28single-precision%29))
  (bind _output_get (Variables|Default|SetTemp (Math|Float|Clamp(Float) (+ (Variables|Default|GetTemp) (* (Variables|Default|GetIncrementValue) (Variables|Default|GetModifier))))))
  (Rendering|Material|SetScalarParameterValue "/Game/_Sandbox/PostProcessing/C_EffectsParameters.C_EffectsParameters" "IsAbsorbing" _output_get :!class /Script/Engine.KismetMaterialLibrary))

(event Collision|EventActorBeginOverlap
  (params (OtherActor :type Actor%20Object%20Reference))
  (Utilities|Casting|CastToMaxence_SandboxCharacter OtherActor)
  (bind _returnvalue (Rendering|Material|GetScalarParameterValue "/Game/_Sandbox/PostProcessing/C_EffectsParameters.C_EffectsParameters" "IsAbsorbing" :!class /Script/Engine.KismetMaterialLibrary))
  (Variables|Default|SetTemp _returnvalue)
  (Variables|Default|SetModifier 1.0))

(event Collision|EventActorEndOverlap
  (params (OtherActor :type Actor%20Object%20Reference))
  (Utilities|Casting|CastToMaxence_SandboxCharacter OtherActor)
  (bind _returnvalue (Rendering|Material|GetScalarParameterValue "/Game/_Sandbox/PostProcessing/C_EffectsParameters.C_EffectsParameters" "IsAbsorbing" :!class /Script/Engine.KismetMaterialLibrary))
  (Variables|Default|SetTemp _returnvalue)
  (Variables|Default|SetModifier -1.0)
  (Sequencer|Player|Play (Variables|/Script/LevelSequence.LevelSequenceActor|GetSequencePlayer (Variables|Default|GetDoorSequence)) :!class /Script/MovieScene.MovieSceneSequencePlayer))

(fn ConstructionScript)